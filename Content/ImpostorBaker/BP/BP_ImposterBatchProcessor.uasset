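; Batch driver that bakes impostor assets for checked actors across configured batch groups.
; BakeImposters finds the "Baker"-tagged sprite generator, then feeds it each StaticMeshActor with its group's frame, resolution, light and asset path settings.
; The baker renders frames and creates or overwrites assets, then its procedural mesh becomes a static mesh passed to FBX export.
; The construction script also finds the baker and calls its scene light toggle.
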(event Custom|Bake%20Imposters
  ;[1 1 1] 从场景中获取ImposterBaker
  (Utilities|IsValid (Variables|Default|GetBaker)
    (:Is%20Valid
      _)
    (:Is%20Not%20Valid
      (bind _outactors (Actor|GetAllActorswithTag "Baker"))
      (for _array_element _outactors
        (bind _asbp_generate_imposter_sprites_seria (Utilities|Casting|CastToBP_Generate_ImposterSpritesSeria _array_element))
        (Variables|Default|SetBaker _asbp_generate_imposter_sprites_seria))))
  ;[1 1 1] 对于每个BatchGroup中的每个状态为勾选的Actor，依次烘焙
  (for _array_element_2 (Variables|Default|GetmBatchGroups)
    (bind _keys (Utilities|Map|Keys (.ActorsToBake (Utilities|Struct|BreakBatchGroup _array_element_2))))
    (for _array_element_3 _keys
      (if (.Value (Utilities|Map|Find (.ActorsToBake (Utilities|Struct|BreakBatchGroup _array_element_2)) _array_element_3))
        (Variables|Default|SetActor (Variables|Default|GetActor))
        ;[1 1 1] Set Baking Actor
        (bind _asstatic_mesh_actor (Utilities|Casting|CastToStaticMeshActor _array_element_3))
        (Variables|/ImpostorBaker/ImpostorBaker/BP/BP_Generate_ImposterSpritesSeria.BP_Generate_ImposterSpritesSeria_C|SetStatic%20Mesh%20Actor (Variables|Default|GetBaker) _asstatic_mesh_actor)
        ;[1 1 1] Set Baking Parameters
        (Variables|/ImpostorBaker/ImpostorBaker/BP/BP_Generate_ImposterSpritesSeria.BP_Generate_ImposterSpritesSeria_C|SetFrames%20XY (Variables|Default|GetBaker) (.FrameX (Utilities|Struct|BreakBatchGroup _array_element_2)))
        (Variables|/ImpostorBaker/ImpostorBaker/BP/BP_Generate_ImposterSpritesSeria.BP_Generate_ImposterSpritesSeria_C|SetResolution (Variables|Default|GetBaker) (.TextureResolution (Utilities|Struct|BreakBatchGroup _array_element_2)))
        (Variables|/ImpostorBaker/ImpostorBaker/BP/BP_Generate_ImposterSpritesSeria.BP_Generate_ImposterSpritesSeria_C|SetScene%20Capture%20Resolution (Variables|Default|GetBaker) (.SceneCaptureResolution (Utilities|Struct|BreakBatchGroup _array_element_2)))
        (bind _returnvalue (Class|ImposterBatchProcessor|GetAssetsPath (.GroupName (Utilities|Struct|BreakBatchGroup _array_element_2)) (Utilities|GetDisplayName _array_element_3)))
        (Variables|/ImpostorBaker/ImpostorBaker/BP/BP_Generate_ImposterSpritesSeria.BP_Generate_ImposterSpritesSeria_C|SetNew%20Asset%20Path (Variables|Default|GetBaker) (.Path (Utilities|Struct|BreakBatchAssetsStr _returnvalue)))
        (Variables|/ImpostorBaker/ImpostorBaker/BP/BP_Generate_ImposterSpritesSeria.BP_Generate_ImposterSpritesSeria_C|SetNew%20Asset%20Texture%20Prefix (Variables|Default|GetBaker) (.TexturePrefix (Utilities|Struct|BreakBatchAssetsStr _returnvalue)))
        (Variables|/ImpostorBaker/ImpostorBaker/BP/BP_Generate_ImposterSpritesSeria.BP_Generate_ImposterSpritesSeria_C|SetNew%20Asset%20MIC%20Name (Variables|Default|GetBaker) (.MICName (Utilities|Struct|BreakBatchAssetsStr _returnvalue)))
        (if (Utilities|Array|ContainsItem (Variables|/ImpostorBaker/ImpostorBaker/BP/BP_Generate_ImposterSpritesSeria.BP_Generate_ImposterSpritesSeria_C|GetMaps%20to%20Render (Variables|Default|GetBaker)) "NewEnumerator10")
          _
          (else
            (Utilities|Array|Add (Variables|/ImpostorBaker/ImpostorBaker/BP/BP_Generate_ImposterSpritesSeria.BP_Generate_ImposterSpritesSeria_C|GetMaps%20to%20Render (Variables|Default|GetBaker)) "NewEnumerator10")))
        (Variables|/ImpostorBaker/ImpostorBaker/BP/BP_Generate_ImposterSpritesSeria.BP_Generate_ImposterSpritesSeria_C|SetLightStates (Variables|Default|GetBaker) (.LightsToBake (Utilities|Struct|BreakBatchGroup _array_element_2)))
        ;[1 1 1] Bake Operations
        (Default|ClearRenderTargets (Variables|Default|GetBaker))
        (Default|2)RenderFrames (Variables|Default|GetBaker))
        (if (Class|BlueprintPathsLibrary|FileExists)
          (Default|4)OverwriteExistingAssets (Variables|Default|GetBaker))
          (else
            (Default|3)CreateStaticAssets (Variables|Default|GetBaker))))
        (bind _returnvalue_2 (Class|ImposterBatchProcessor|CreateStaticMesh (Variables|/ImpostorBaker/ImpostorBaker/BP/BP_Generate_ImposterSpritesSeria.BP_Generate_ImposterSpritesSeria_C|GetProceduralMesh (Variables|Default|GetBaker)) (Utilities|GetDisplayName _array_element_3)))
        (Class|ImposterBatchProcessor|OutputFBX _returnvalue_2)))))

(event EventBeginPlay)

(event Collision|EventActorBeginOverlap
  (params (OtherActor :type Actor%20Object%20Reference)))

(event EventTick
  (params (DeltaSeconds :type Float%20%28single-precision%29)))

(fn ConstructionScript
  ;[1 1 1] 从场景中获取ImposterBaker(是一个BP_Generate_ImposterSprites类）
  (Utilities|IsValid (Variables|Default|GetBaker)
    (:Is%20Valid
      _)
    (:Is%20Not%20Valid
      (bind _outactors (Actor|GetAllActorswithTag "Baker"))
      (for _array_element _outactors
        (bind _asbp_generate_imposter_sprites_seria (Utilities|Casting|CastToBP_Generate_ImposterSpritesSeria _array_element))
        (Variables|Default|SetBaker _asbp_generate_imposter_sprites_seria))))
  (Default|ToggleSceneLightFunc (Variables|Default|GetBaker) true))